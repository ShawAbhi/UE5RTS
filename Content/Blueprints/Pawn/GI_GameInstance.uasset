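; Game instance that manages the PlayFab session and the local SG_TempLocal save game.
; Init loads any existing save and logs in with hardcoded credentials; Shutdown writes the save back.
; Login success fetches user data and inventory, broadcasting each result on GameplayMessageSubsystem channels.
; It also offers registration, user data updates, spawnable-struct accessors and a fixed currency value, alongside disconnected test snippets.
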(event `Login_Failed`
  (params (error :type "PlayFabError Structure") (customData :type "Object Object Reference"))
  ;[0.4531 0.3257 0.3257 0.663] Log Failed Events
  (`self.PrintFailedCalls` "Login Failed :  " error))

(event `Registeration_Failed`
  (params (error :type "PlayFabError Structure") (customData :type "Object Object Reference"))
  ;[0.4531 0.3257 0.3257 0.663] Log Failed Events
  (`self.PrintFailedCalls` "Register Failed : " error))

(event `Playfab_Failed`
  (params (error :type "PlayFabError Structure") (customData :type "Object Object Reference"))
  ;[0.4531 0.3257 0.3257 0.663] Log Failed Events
  (`self.PrintFailedCalls` "" error))

(event `CE_CloudFunction_Success`
  (params (result :type "ClientExecuteCloudScriptResult Structure") (customData :type "Object Object Reference"))
  ;[0.1417 0.2243 0.3125 0.346 35] Sample Cloud script
  (`KismetSystemLibrary.PrintString` "CE_CloudDunction Success"))

(event `PrintFailedCalls`
  (params (`Append Message` :type String :default " ") (PlayFabError :type "PlayFabError Structure (by ref)"))
  (bind (_haserror _errorcode _errorname _errormessage) (break `PlayFabError` PlayFabError))
  ;[0.4531 0.3257 0.3257 0.663] Log Failed Events
  (`KismetSystemLibrary.PrintString` (`KismetStringLibrary.Concat_StrStr` `Append Message` _errorname "  :  " _errormessage " #1211") true true (struct :`R` 0.510417 :`G` 0.003995 :`A` 1.0) 20.0))

(event `self.ReceiveShutdown`
  (`self.SaveGame`))

(event `self.ReceiveInit`
  (`self.InitSaveGame`)
  (`self.Try_Login` "theuser" "ExampleSecret"))

(event `Try_Login`
  (params (Username :type String) (Password :type String))
  (`PlayFabClientAPI.LoginWithPlayFab` (make `ClientLoginWithPlayFabRequest` null null Password Username) (`|CreateDelegate` :!event `Login_Success`) (`|CreateDelegate` :!event `Login_Failed`)))

(event `Try_Register`
  (params (Username :type String) (Email :type String) (Password :type String))
  (`PlayFabClientAPI.RegisterPlayFabUser` (make `ClientRegisterPlayFabUserRequest` null Username Email "" null Password "" true Username) (`|CreateDelegate` :!event `Register_Successful`) (`|CreateDelegate` :!event `Registeration_Failed`)))

(event `Login_Success`
  (params (result :type "ClientLoginResult Structure") (customData :type "Object Object Reference"))
  (bind _output_get (set `self.LoginResult` result))
  (set `self.bIsLoggedIn` true)
  (`GameplayMessageSubsystem.K2_BroadcastMessage` (subsystem `GameplayMessageSubsystem`) (struct :`TagName` "Message.Playfab.Login.Init") _output_get)
  (`self.CE_GetUserData`)
  (`self.GetUserInventory`))

(event `Register_Successful`
  (params (result :type "ClientRegisterPlayFabUserResult Structure") (customData :type "Object Object Reference"))
  (set `self.RegisteredResult` result))

(event `CE_GetUserData`
  (bind ((`PlayFabId` _playfabid) (`AuthenticationContext` _authenticationcontext)) (break `ClientLoginResult` (`self.LoginResult`)))
  ;[0.03812 0.1615 0.1502 0.496 35] API Calls (Get)
  (`PlayFabClientAPI.GetUserData` (make `ClientGetUserDataRequest` 0 "" _playfabid _authenticationcontext) (delegate `UserData_Success`) (`|CreateDelegate` :!event `Playfab_Failed`)))

(event `UserData_Success`
  (params (result :type "ClientGetUserDataResult Structure") (customData :type "Object Object Reference"))
  ;[0.03812 0.1615 0.1502 0.496 35] API Calls (Get)
  (bind _output_get (set `self.UserData` result))
  (`GameplayMessageSubsystem.K2_BroadcastMessage` (subsystem `GameplayMessageSubsystem`) (struct :`TagName` "Message.Playfab.Login.UserData.Init") _output_get))

(event `GetUserInventory`
  ;[0.03812 0.1615 0.1502 0.496 35] API Calls (Get)
  (`PlayFabClientAPI.GetUserInventory` (make `ClientGetUserInventoryRequest` null (`.AuthenticationContext` (break `ClientLoginResult` (`self.LoginResult`)))) (delegate `CustomEvent`) (`|CreateDelegate` :!event `Playfab_Failed`)))

(event `CustomEvent`
  (params (result :type "ClientGetUserInventoryResult Structure") (customData :type "Object Object Reference"))
  ;[0.03812 0.1615 0.1502 0.496 35] API Calls (Get)
  (bind _output_get (set `self.UserInventory` result))
  (`GameplayMessageSubsystem.K2_BroadcastMessage` (subsystem `GameplayMessageSubsystem`) (struct :`TagName` "Message.Playfab.Login.UserInventory.Init") _output_get))

(event `/Game/Blueprints/Pawn/BPI_GameInstanceInterface.UpdateUserData`
  (params (Data :type "PlayFabJsonObject Object Reference"))
  ;[0.03812 0.1615 0.1502 0.496 35] API Calls (Get)
  (`PlayFabClientAPI.UpdateUserData` (make `ClientUpdateUserDataRequest` null Data "" "pfenum_Public" (`.AuthenticationContext` (break `ClientLoginResult` (`self.LoginResult`)))) (delegate `UserDataUpdated`) (`|CreateDelegate` :!event `Playfab_Failed`)))

(event `UserDataUpdated`
  (params (result :type "ClientUpdateUserDataResult Structure") (customData :type "Object Object Reference"))
  ;[0.03812 0.1615 0.1502 0.496 35] API Calls (Get)
  (`KismetSystemLibrary.PrintString` "User Data Updated"))

(fn `CreateDefaultSaveGame`
  (bind _returnvalue (`GameplayStatics.CreateSaveGameObject` "/Game/Blueprints/Pawn/SG_TempLocal.SG_TempLocal_C"))
  (`GameplayStatics.SaveGameToSlot` _returnvalue (`self.Slot Name`))
  (set `self.SaveGameRef` _returnvalue))

(fn `GetCurrencyValue`
  (returns (Currency :type Integer))
  (return 50000))

(fn `GetSpawnableStructElement`
  (params (Index :type Integer))
  (returns (Output :type "/Game/Data/Spawnables/FSpawnables Structure (by ref)"))
  (return (`|GetArrayItem` (`/Game/Blueprints/Pawn/SG_TempLocal.SpawnableStruct` (`self.SaveGameRef`)) Index)))

(fn `InitSaveGame`
  (bind _returnvalue (`GameplayStatics.DoesSaveGameExist` (`self.Slot Name`)))
  (bind _output_get (set `self.SG_Found?` _returnvalue))
  (if _output_get
    (bind _returnvalue_2 (`GameplayStatics.LoadGameFromSlot` (`self.Slot Name`)))
    (`/Engine/EditorBlueprintResources/StandardMacros.IsValid` _returnvalue_2
      (:`Is Valid`
        (bind _assg_temp_local (cast `/Game/Blueprints/Pawn/SG_TempLocal` _returnvalue_2))
        (set `self.SaveGameRef` _assg_temp_local)))))

(fn `LogDataValue`
  (params (InputPin :type "PlayFabJsonObject Object Reference"))
  (bind _returnvalue (`EasyJsonParseManager.LoadFromString` (`PlayFabJsonObject.EncodeJson` InputPin))
    (:`Successed`
      (for _array_element (`PlayFabJsonObject.GetFieldNames` InputPin)
        (`KismetSystemLibrary.PrintString` (`KismetStringLibrary.Concat_StrStr` _array_element " ::  " (`EasyJsonObject.ReadString` _returnvalue (`KismetStringLibrary.Concat_StrStr` _array_element ".value") "")) true false (struct :`G` 0.022378 :`B` 0.067708 :`A` 1.0) 10.0)))))

(fn `SaveGame`
  (`GameplayStatics.SaveGameToSlot` (`self.SaveGameRef`) (`self.Slot Name`)))

(fn `UpdateSpawnableStruct`
  (params (Item :type "/Game/Data/Spawnables/FSpawnables Structure (by ref)") (Index :type Integer))
  (`KismetArrayLibrary.Array_Set` (`/Game/Blueprints/Pawn/SG_TempLocal.SpawnableStruct` (`self.SaveGameRef`)) Index Item))