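; BP_SpawnAble is a data-driven spawnable actor with a name plate and a controls widget.
; The construction script writes the actor's location into Data as a 2D position in meters.
; BeginPlay applies Data's name, position, quarter-turn orientation and bounding scale, then async-loads the base mesh, with a blocking load if the cast fails.
; Ghost mode toggles controls visibility, and a getter exposes the bounding mesh's scale and location.
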(event `self.ReceiveBeginPlay`
  (bind (_data_index _data_name _data_position _data_scale _data_orientation) (break `/Game/Data/Spawnables/FSpawnables` (`self.Data`)))
  (bind ((`Index_20_A40983864534F9E78D81B68A2BDC4066` _index) (`Scale_21_BB7A2B314950A9261101FAAA373639B3` _scale) (`BaseMesh_13_421FF8E5465B6D87B4597BA7BF045EAC` _basemesh)) (break `/Game/Data/Spawnables/FSpawnables` (`self.Data`)))
  (`|ExecutionSequence`
    (:`then_0`
      (bind _aswbp_name_plate (cast `/Game/Data/Spawnables/WBP_NamePlate` (`WidgetComponent.GetWidget` (`self.Name`))))
      (set `TextBlock.Text` (`KismetTextLibrary.Conv_StringToText` _data_name) (`/Game/Data/Spawnables/WBP_NamePlate.Text` _aswbp_name_plate))
      (`self.K2_SetActorLocationAndRotation` (`KismetMathLibrary.Conv_Vector2DToVector` (* _data_position 100.0)) (`KismetMathLibrary.MakeRotator` 0.0 0.0 (`KismetMathLibrary.Conv_IntToDouble` (* _data_orientation 90))))
      (`SceneComponent.SetWorldScale3D` (`self.BoundingMesh`) _data_scale)
      (bind _object (`|LoadAsset` _basemesh)
        (:`Completed`
          (bind _asstatic_mesh (cast `StaticMesh` _object)
            (:`then`
              (`StaticMeshComponent.SetStaticMesh` (`self.BaseMesh`) _asstatic_mesh))
            (:`CastFailed`
              (bind _returnvalue (`KismetSystemLibrary.LoadAsset_Blocking` _basemesh))
              (bind _asstatic_mesh_2 (cast `StaticMesh` _returnvalue))
              (`StaticMeshComponent.SetStaticMesh` (`self.BaseMesh`) _asstatic_mesh_2))))))
    (:`then_1`
      (bind _aswbp_spawnable_controls (cast `/Game/Blueprints/UI/Widgets/EditMode/WBP_SpawnableControls` (`WidgetComponent.GetWidget` (`self.Controls`))))
      (set `self.As WBP Spawnable Controls` _aswbp_spawnable_controls))))

(event `CE_GhostMode`
  (params (Enable :type Boolean))
  (bind _output_get (set `self.GhostMode` Enable))
  (`SceneComponent.SetVisibility` (`self.Controls`) _output_get false))

(fn `GetBoundingScaleLocation`
  (returns (Scale :type "Vector Structure") (Location :type "Vector Structure"))
  (bind _boundingmesh (`self.BoundingMesh`))
  (return (`SceneComponent.K2_GetComponentScale` _boundingmesh) (`SceneComponent.K2_GetComponentLocation` _boundingmesh)))

(fn `UserConstructionScript`
  (bind (_data_index _data_name _data_position _data_scale _data_orientation _data_basemesh) (break `/Game/Data/Spawnables/FSpawnables` (`self.Data`)))
  (set `self.Data` (make `/Game/Data/Spawnables/FSpawnables` _data_index _data_name (/ (`KismetMathLibrary.Conv_VectorToVector2D` (`self.K2_GetActorLocation`)) 100.0) _data_scale _data_orientation _data_basemesh)))